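; BP_Door is a double level door that swings open when the player's BP_Maria has the matching key.
; An overlap on LevelDoorCollider compares Maria's MariaHasLevelKey with the key in the door's LevelDoors data, read by casting itself to DoorInTheLevel.
; On a match, a timeline rotates the left and right pivots in yaw and fires an event track that plays the opening sound in 2D.
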(event `self.LevelDoorCollider.OnComponentBeginOverlap`
  (params (OverlappedComponent :type "PrimitiveComponent Object Reference") (OtherActor :type "Actor Object Reference") (OtherComp :type "PrimitiveComponent Object Reference") (OtherBodyIndex :type Integer) (bFromSweep :type Boolean) (SweepResult :type "HitResult Structure (by ref)"))
  (bind _asbp_maria (cast `/Game/Characters/Maria/BP/BP_Maria` (`GameplayStatics.GetPlayerPawn` 0)))
  (bind _asdoor_in_the_level (cast `/Game/Blueprints/DoorInTheLevel` self))
  (bind _leveldoors_whatkeyisit_ (break `/Game/items/structures/structure_levelDoors` (`/Game/Blueprints/DoorInTheLevel.levelDoors` _asdoor_in_the_level)))
  (if (`|EnumEquality` (`/Game/Characters/Maria/BP/BP_Maria.MariaHasLevelKey` _asbp_maria) _leveldoors_whatkeyisit_)
    (bind (_direction _rotationldoor _rotationrdoor) (`Timeline|Timeline_0`)
      (:`Update`
        (`SceneComponent.K2_SetRelativeRotation` (`self.RightDoorPivot`) (`KismetMathLibrary.MakeRotator` 0.0 0.0 _rotationrdoor) false false)
        (`SceneComponent.K2_SetRelativeRotation` (`self.LeftDoorPivot`) (`KismetMathLibrary.MakeRotator` 0.0 0.0 _rotationldoor) false false))
      (:`playSound`
        (`GameplayStatics.PlaySound2D` "/Game/sounds/doorOpens.doorOpens" 1.0 1.0 0.0 null null)))))

(fn `UserConstructionScript`)