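; World pickup item that BP_Maria collects into her items by pressing G.
; Construction looks up the item enum's row in Items_table, merges in the quantity and sets the mesh; BeginPlay passes that info to the widget.
; Box overlap toggles input, and G adds the item, plays a pickup montage and destroys the actor if it is Maria's SelectedItem.
; SelectedItem toggles custom-depth rendering and widget visibility.
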(event `self.ReceiveBeginPlay`
  (bind _aswb_info_item (cast `/Game/UI/WB_infoItem` (`WidgetComponent.GetUserWidgetObject` (`self.Widget`))))
  (set `/Game/UI/WB_infoItem.info_widged` (`self.information_complete`) _aswb_info_item))

(event `self.Box.OnComponentBeginOverlap`
  (params (OverlappedComponent :type "PrimitiveComponent Object Reference") (OtherActor :type "Actor Object Reference") (OtherComp :type "PrimitiveComponent Object Reference") (OtherBodyIndex :type Integer) (bFromSweep :type Boolean) (SweepResult :type "HitResult Structure (by ref)"))
  (cast `/Game/Characters/Maria/BP/BP_Maria` OtherActor)
  (`self.EnableInput` (`GameplayStatics.GetPlayerController` 0))
  (set `self.nearCharacter` true))

(event `self.Box.OnComponentEndOverlap`
  (params (OverlappedComponent :type "PrimitiveComponent Object Reference") (OtherActor :type "Actor Object Reference") (OtherComp :type "PrimitiveComponent Object Reference") (OtherBodyIndex :type Integer))
  (cast `/Game/Characters/Maria/BP/BP_Maria` OtherActor)
  (`self.DisableInput` (`GameplayStatics.GetPlayerController` 0))
  (set `self.nearCharacter` false))

(event `Key|G`
  (params (Key :type "Key Structure"))
  (bind _returnvalue (`GameplayStatics.GetPlayerPawn` 0))
  (:`Pressed`
    (`GameplayStatics.PlaySound2D` "/Game/sounds/384867__ali-6868__right-grass-grassy-footstep-2.384867__ali-6868__right-grass-grassy-footstep-2" 1.0 1.0 0.0 null null)
    (bind _asbp_maria (cast `/Game/Characters/Maria/BP/BP_Maria` _returnvalue))
    (if (== (`/Game/Characters/Maria/BP/BP_Maria.selectedItem` _asbp_maria) self)
      (`/Game/Characters/Maria/BP/BP_Maria.addItem` _asbp_maria (`self.information_complete`))
      (bind _asbp_maria_2 (cast `/Game/Characters/Maria/BP/BP_Maria` _returnvalue))
      (`Character.PlayAnimMontage` _asbp_maria_2 "/Game/Characters/Maria/animations/PickFruit_montage.PickFruit_montage" 1.0 "None")
      (`self.K2_DestroyActor`))))

(fn `getCompleteInfo`
  (params (itemInfo :type "/Game/items/structures/structure_item Structure"))
  (returns (itemCompleteInfo :type "/Game/items/structures/structure_item_complete Structure"))
  (bind _returnvalue (`|GetDataTableRow` "/Game/items/structures/Items_table.Items_table" (`KismetStringLibrary.Conv_StringToName` (`|GetEnumeratorNameAsString` itemInfo_Item_2_F451C3D14F7DB07C6DFEEBBF8573EAAC)))
    (:`then`
      (bind _structout (setmembers `/Game/items/structures/structure_item_complete` :`StructRef` _returnvalue :`quantity` itemInfo_quantity_5_F913059249EA77E54CDF829450FB972A))
      (return _structout))))

(fn `selectedItem`
  (params (Selected :type Boolean))
  (`PrimitiveComponent.SetRenderCustomDepth` (`self.model`) Selected)
  (`SceneComponent.SetVisibility` (`self.Widget`) (`local.Selected`) false))

(fn `UserConstructionScript`
  (bind _itemcompleteinfo (`self.getCompleteInfo` (`self.info`)))
  (bind _output_get (set `self.information_complete` _itemcompleteinfo))
  (`StaticMeshComponent.SetStaticMesh` (`self.model`) (`.model_28_7EC9478D41B0D08726BABDB7D8273312` (break `/Game/items/structures/structure_item_complete` _output_get))))